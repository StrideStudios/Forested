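; Construction-script Blueprint that orients the actor by converting its Lat and Yaw values into a rotation using spherical trigonometry.
; Roll is the arcsine of cos(Lat) times sin(Yaw).
; World yaw comes from an arccosine of that roll angle and Lat, resembling a horizon hour-angle formula.
; The sign of Yaw selects between two mirrored offsets to resolve the arccosine's ambiguity.
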(fn `UserConstructionScript`
  (bind _returnvalue (`KismetMathLibrary.DegAsin` (* (`KismetMathLibrary.DegCos` (`self.Lat`)) (`KismetMathLibrary.DegSin` (`self.Yaw`)))))
  (bind _returnvalue_2 (`KismetMathLibrary.DegAcos` (/ (- 0.0 (* (`KismetMathLibrary.DegSin` _returnvalue) (`KismetMathLibrary.DegSin` (`self.Lat`)))) (* (`KismetMathLibrary.DegCos` _returnvalue) (`KismetMathLibrary.DegCos` (`self.Lat`))))))
  (`self.K2_SetActorRotation` (`KismetMathLibrary.MakeRotator` _returnvalue 0.0 (`KismetMathLibrary.SelectFloat` (+ _returnvalue_2 180.0) (- 540.0 _returnvalue_2) (> (`self.Yaw`) 0.0)))))