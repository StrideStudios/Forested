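; Chopping stump that holds a single log item and splits it when hit with axe damage.
; Inserting an item async-loads and shows its mesh; removing it hides the mesh and disables collision.
; Full logs snap to the player's facing and become two elm halves; halves become quarters only when struck along the required axis.
; Dot products set the piece orientation flags, and pieces spawn flying apart sideways with opposite spin.
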(event `DamageableInterface.Damage`
  (params (Player :type "FPlayer Object Reference") (HitResult :type "HitResult Structure (by ref)") (Damage :type "Float (single-precision)") (DamageType :type "EDamageType Enum" :default "Basic"))
  (bind (_outitem _returnvalue) (`InventoryBase.ReceiveGetItem` 0))
  (if _returnvalue
    (bind _treelogtype (message `ChopStumpInterface.GetChopStumpProperties` (`ItemLibrary.Top` _outitem)))
    (if (`|EnumEquality` DamageType "Axe")
      (switch `ETreeLogType` _treelogtype
        (:`Full`
          (`self.SliceFullLog` Player))
        (:`Half`
          (`self.SliceHalfLog` Player))))))

(event `SliceFullLog`
  (params (Player :type "FPlayer Object Reference"))
  (bind _returnvalue (`self.K2_GetActorRotation` Player))
  (bind _returnvalue_2 (`FPlayer.GetPlayerForwardVector` Player))
  (bind _inverted (`self.Inverted`))
  (bind _isy (`self.IsY`))
  (bind _staticmesh2 (`self.StaticMesh2`))
  (bind _returnvalue_3 (`SceneComponent.K2_GetComponentToWorld` _staticmesh2))
  (bind _returnvalue_4 (* (`FPlayer.GetPlayerForwardVector` Player) -200.0))
  (bind _returnvalue_5 (* (`FPlayer.GetPlayerRightVector` Player) 150.0))
  (bind _returnvalue_6 (`KismetMathLibrary.Dot_VectorVector` _returnvalue_2 (`SceneComponent.GetRightVector` (`self.StaticMesh2`))))
  (bind _returnvalue_7 (`KismetMathLibrary.SelectRotator` _returnvalue (`KismetMathLibrary.ComposeRotators` _returnvalue (struct :`Yaw` -90.0)) (`self.IsY`)))
  (bind _returnvalue_8 (`KismetMathLibrary.Dot_VectorVector` _returnvalue_2 (`SceneComponent.GetForwardVector` (`self.StaticMesh2`))))
  (set `self.IsY` (< (`KismetMathLibrary.Abs` _returnvalue_6) (`KismetMathLibrary.Abs` _returnvalue_8)))
  (set `self.Inverted` (> (`KismetMathLibrary.SelectFloat` _returnvalue_6 _returnvalue_8 (`self.IsY`)) 0.0))
  (`SceneComponent.K2_SetWorldRotation` _staticmesh2 (`KismetMathLibrary.SelectRotator` _returnvalue_7 (`KismetMathLibrary.ComposeRotators` _returnvalue_7 (struct :`Yaw` 180.0)) (`self.Inverted`)) false false)
  (`|ExecutionSequence`
    (:`then_0`
      (bind _returnvalue_9 (`|ConstructItem` "/Game/Blueprints/Items/Trees/Elm/BP_ElmLogHalf.BP_ElmLogHalf_C" _inverted _isy))
      (`ItemActorSpawnAsyncAction.SpawnItemActor` _returnvalue_3 _returnvalue_9 _returnvalue_5 _returnvalue_4))
    (:`then_1`
      (bind _returnvalue_10 (`|ConstructItem` "/Game/Blueprints/Items/Trees/Elm/BP_ElmLogHalf.BP_ElmLogHalf_C" (not _inverted) _isy))
      (`ItemActorSpawnAsyncAction.SpawnItemActor` _returnvalue_3 _returnvalue_10 (* _returnvalue_5 -1.0) (* _returnvalue_4 -1.0)))
    (:`then_2`
      (`InventoryBase.RemoveItem` 0))))

(event `SliceHalfLog`
  (params (Player :type "FPlayer Object Reference"))
  (bind _returnvalue (`FPlayer.GetPlayerForwardVector` Player))
  (bind _returnvalue_2 (`SceneComponent.K2_GetComponentToWorld` (`self.StaticMesh2`)))
  (bind _returnvalue_3 (* _returnvalue -200.0))
  (bind _returnvalue_4 (* (`FPlayer.GetPlayerRightVector` Player) 150.0))
  (bind _returnvalue_5 (* _returnvalue_4 -1.0))
  (bind _returnvalue_6 (* _returnvalue_3 -1.0))
  (bind _asbp_elm_log_half (cast `/Game/Blueprints/Items/Trees/Elm/BP_ElmLogHalf` (`ItemLibrary.Top` (`InventoryBase.ReceiveGetItem` 0))))
  (bind _isy (`/Game/Blueprints/Items/Trees/Elm/BP_ElmLogHalf.IsY` _asbp_elm_log_half))
  (bind _returnvalue_7 (`KismetMathLibrary.Dot_VectorVector` _returnvalue (`KismetMathLibrary.SelectVector` (`SceneComponent.GetRightVector` (`self.StaticMesh2`)) (`SceneComponent.GetForwardVector` (`self.StaticMesh2`)) _isy)))
  (if (> (`KismetMathLibrary.Abs` _returnvalue_7) 0.9)
    (`|ExecutionSequence`
      (:`then_0`
        (if _isy
          (bind _returnvalue_8 (> _returnvalue_7 0.0))
          (bind _isnegativehalf (`/Game/Blueprints/Items/Trees/Elm/BP_ElmLogHalf.IsNegativeHalf` _asbp_elm_log_half))
          (bind _returnvalue_9 (`|ConstructItem` "/Game/Blueprints/Items/Trees/Elm/BP_ElmLogQuarter.BP_ElmLogQuarter_C" _returnvalue_8 _isnegativehalf))
          (`ItemActorSpawnAsyncAction.SpawnItemActor` _returnvalue_2 _returnvalue_9 _returnvalue_4 _returnvalue_3)
          (else
            (bind _returnvalue_10 (`|ConstructItem` "/Game/Blueprints/Items/Trees/Elm/BP_ElmLogQuarter.BP_ElmLogQuarter_C" _isnegativehalf _returnvalue_8))
            (`ItemActorSpawnAsyncAction.SpawnItemActor` _returnvalue_2 _returnvalue_10 _returnvalue_4 _returnvalue_3))))
      (:`then_1`
        (if _isy
          (bind _returnvalue_11 (not _returnvalue_8))
          (bind _returnvalue_12 (`|ConstructItem` "/Game/Blueprints/Items/Trees/Elm/BP_ElmLogQuarter.BP_ElmLogQuarter_C" _returnvalue_11 _isnegativehalf))
          (`ItemActorSpawnAsyncAction.SpawnItemActor` _returnvalue_2 _returnvalue_12 _returnvalue_5 _returnvalue_6)
          (else
            (bind _returnvalue_13 (`|ConstructItem` "/Game/Blueprints/Items/Trees/Elm/BP_ElmLogQuarter.BP_ElmLogQuarter_C" _isnegativehalf _returnvalue_11))
            (`ItemActorSpawnAsyncAction.SpawnItemActor` _returnvalue_2 _returnvalue_13 _returnvalue_5 _returnvalue_6))))
      (:`then_2`
        (`InventoryBase.RemoveItem` 0)))))

(event `self.ReceiveOnInsertItem`
  (params (Item :type "ItemHeap Structure") (Slot :type Integer))
  (bind (_treelogtype _staticmesh) (message `ChopStumpInterface.GetChopStumpProperties` (`ItemLibrary.Top` Item)))
  (bind _object (`LoadSoftPtrAsyncAction.LoadPtrAsync` _staticmesh)
    (:`then`
      (bind _asstatic_mesh (cast `StaticMesh` _object))
      (`StaticMeshComponent.SetStaticMesh` (`self.StaticMesh2`) _asstatic_mesh)
      (`SceneComponent.SetVisibility` (`self.StaticMesh2`) true false)
      (`PrimitiveComponent.SetCollisionEnabled` (`self.StaticMesh2`) "QueryAndPhysics"))))

(event `self.ReceiveOnRemoveItem`
  (params (Item :type "ItemHeap Structure") (Slot :type Integer))
  (bind _staticmesh2 (`self.StaticMesh2`))
  (`SceneComponent.SetVisibility` _staticmesh2 false false)
  (`PrimitiveComponent.SetCollisionEnabled` _staticmesh2 "NoCollision"))

(fn `CanSelect`
  (params (Player :type "FPlayer Object Reference") (HitResult :type "HitResult Structure (by ref)") (HeldTime :type "Float (double-precision)"))
  (returns (ReturnValue :type Boolean))
  (return (and (`parent.CanSelect` Player HitResult HeldTime) (== (`.HitComponent` (`GameplayStatics.BreakHitResult` HitResult)) (`self.Box`)))))

(fn `ReceiveCanItemBeInserted`
  (params (Item :type "ItemHeap Structure") (Slot :type Integer))
  (returns (ReturnValue :type Boolean))
  (bind _returnvalue (`parent.ReceiveCanItemBeInserted` Item Slot))
  (return (and _returnvalue (not (`InventoryBase.HasItem` 0)))))

(fn `UserConstructionScript`)