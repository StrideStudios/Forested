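; BP_Sky is a sky actor that configures its Sun and Moon lights and updates light actors in the level.
; Its construction script calls the parent's, sets light function, bloom and occlusion mask values on both lights, then refreshes every EnvironmentLight and TimedLight, passing itself as the sky.
; BeginPlay calls RenderSky, whose event invokes SkySettings, an empty function in this Blueprint.
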(event `self.ReceiveBeginPlay`
  (`self.RenderSky` 0.0))

(event `self.ReceiveRenderSky`
  (params (DeltaTime :type "Float (single-precision)") (Sky :type "Sky Object Reference"))
  (`self.SkySettings`))

(fn `SkySettings`)

(fn `UserConstructionScript`
  (`parent.UserConstructionScript`)
  (`LightComponent.SetLightFunctionDisabledBrightness` (`self.Sun`) 1.0)
  (`LightComponent.SetLightFunctionDisabledBrightness` (`self.Moon`) 1.0)
  (`LightComponent.SetBloomScale` (`self.Moon`) 0.125)
  (`LightComponent.SetBloomScale` (`self.Sun`) 0.125)
  (`DirectionalLightComponent.SetOcclusionMaskDarkness` (`self.Moon`) 0.05)
  (`DirectionalLightComponent.SetOcclusionMaskDarkness` (`self.Sun`) 0.05)
  (`|ExecutionSequence`
    (:`then_0`
      (bind _outactors (`GameplayStatics.GetAllActorsOfClass` "/Script/Forested.EnvironmentLight"))
      (`EnvironmentLight.RefreshLight` _outactors 0.0 self))
    (:`then_1`
      (bind _outactors_2 (`GameplayStatics.GetAllActorsOfClass` "/Script/Forested.TimedLight"))
      (`TimedLight.RefreshLight` _outactors_2 0.0 self))))