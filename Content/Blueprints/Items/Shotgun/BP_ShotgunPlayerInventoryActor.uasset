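; Player inventory actor for the shotgun, handling shooting, aiming, racking and reloading with a viewmodel mesh.
; Shots originate from the viewmodel-converted ShootPoint, which also positions a widget every tick.
; Player and viewmodel montages play in tandem, with rack and reload animations selected by bullet count.
; Shell meshes update visibility from that count, and a BulletEject notify hides the ejected shell.
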(event `self.ReceiveInit`
  (`self.DetermineBulletVisibility`))

(event `self.ReceiveOnLeftInteract`
  (params (IsMontagePlaying :type Boolean))
  (if (`KismetMathLibrary.BooleanNOR` (`PlayerInputComponent.IsHoldingLeftInteract` (`FPlayer.PlayerInputComponent` (`LevelDefaults.GetPlayer`))) (`PlayerAnimInstance.IsAMontageOfAnimationGroupActive` (`self.GetPlayerAnimInstance`) "SecondaryGroup" false))
    (bind _returnvalue (`self.Shoot` "/Game/Geometry/Meshes/Player/Anims/Shotgun/AM_ShotgunShooting.AM_ShotgunShooting" (make `ViewmodelVector` (`ViewmodelSkeletalMeshComponent.GetViewmodelData` (`self.ViewmodelSkeletalMesh`)) (`SceneComponent.K2_GetComponentLocation` (`self.ShootPoint`))) 1.0 0.0 (`PlayerInputComponent.IsHoldingRightInteract` (`FPlayer.PlayerInputComponent` (`LevelDefaults.GetPlayer`)))))
    (if _returnvalue
      (`StartMontageAsyncAction.StartMontage` (`self.ViewmodelSkeletalMesh`) "/Game/Geometry/Meshes/Items/Shotgun/Anims/AM_ShotgunShoot.AM_ShotgunShoot" true))))

(event `self.ReceiveOnRightInteract`
  (params (IsMontagePlaying :type Boolean))
  (`self.Aim` "/Game/Geometry/Meshes/Player/Anims/Shotgun/AM_ShotgunAim.AM_ShotgunAim"))

(event `self.ReceiveOnRightEndInteract`
  (params (IsMontagePlaying :type Boolean))
  (bind _returnvalue (`PlayerAnimInstance.GetCurrentActiveMontageOfAnimationGroup` (`self.GetPlayerAnimInstance`) "PrimaryGroup"))
  (if (== _returnvalue "/Game/Geometry/Meshes/Player/Anims/Shotgun/AM_ShotgunAim.AM_ShotgunAim")
    (`self.UnAim` _returnvalue)))

(event `self.ReceiveTick`
  (params (DeltaSeconds :type "Float (single-precision)"))
  (`self.TransformWidgetToShootPoint` DeltaSeconds (`ViewmodelMeshes.Conv_ViewmodelVectorToVector` (make `ViewmodelVector` (`ViewmodelSkeletalMeshComponent.GetViewmodelData` (`self.ViewmodelSkeletalMesh`)) (`SceneComponent.K2_GetComponentLocation` (`self.ShootPoint`))))))

(event `self.EndShot`
  (bind (_outitem _returnvalue) (`self.GetShootItem`))
  (bind _returnvalue_2 (`PlayerAnimInstance.GetCurrentActiveMontageOfAnimationGroup` (`self.GetPlayerAnimInstance`) "PrimaryGroup"))
  (bind _bullets (`ShootItem.Bullets` _outitem))
  (if _returnvalue
    (bind _outsuccess (`StartMontageAsyncAction.StartMontage` (`Character.Mesh` (`self.GetPlayer`)) "/Game/Geometry/Meshes/Player/Anims/Shotgun/AM_ShotgunRacking.AM_ShotgunRacking" true)
      (:`then`
        (if _outsuccess
          (bind (_outsuccess_2 _notifyname) (`StartMontageAsyncAction.StartMontage` (`self.ViewmodelSkeletalMesh`) (select `bool` (> _bullets 1) :`false` (select `int` _bullets :`0` "/Game/Geometry/Meshes/Items/Shotgun/Anims/AM_ShotgunRackEmpty.AM_ShotgunRackEmpty" :`1` "/Game/Geometry/Meshes/Items/Shotgun/Anims/AM_ShotgunRack.AM_ShotgunRack" :!type "AnimMontage Object Reference") :`true` "/Game/Geometry/Meshes/Items/Shotgun/Anims/AM_ShotgunRackMultiple.AM_ShotgunRackMultiple") true)
            (:`OnBlendOut`
              (`self.DetermineBulletVisibility`)
              (if (`PlayerInputComponent.IsHoldingRightInteract` (`FPlayer.PlayerInputComponent` (`LevelDefaults.GetPlayer`)))
                _
                (elif (== _returnvalue_2 "/Game/Geometry/Meshes/Player/Anims/Shotgun/AM_ShotgunAim.AM_ShotgunAim")
                  (`self.UnAim` _returnvalue_2))))
            (:`OnNotifyBegin`
              (if (== _notifyname "BulletEject")
                (`SceneComponent.SetVisibility` (`self.EjectBullet`) false false)))))))))

(event `self.ReceiveOnReload`
  (params (IsMontagePlaying :type Boolean))
  (bind (_outitem _returnvalue) (`self.GetShootItem`))
  (bind _bullets (`ShootItem.Bullets` _outitem))
  (if _returnvalue
    (if (not (`PlayerInputComponent.IsHoldingReload` (`FPlayer.PlayerInputComponent` (`LevelDefaults.GetPlayer`))))
      (bind _outsuccess (`StartMontageAsyncAction.StartMontage` (`self.ViewmodelSkeletalMesh`) (select `int` _bullets :`0` "/Game/Geometry/Meshes/Items/Shotgun/Anims/Reload/AM_Shotgun_ReloadFull.AM_Shotgun_ReloadFull" :`1` "/Game/Geometry/Meshes/Items/Shotgun/Anims/Reload/AM_Shotgun_Reload5.AM_Shotgun_Reload5" :`2` "/Game/Geometry/Meshes/Items/Shotgun/Anims/Reload/AM_Shotgun_Reload4.AM_Shotgun_Reload4" :`3` "/Game/Geometry/Meshes/Items/Shotgun/Anims/Reload/AM_Shotgun_Reload3.AM_Shotgun_Reload3" :`4` "/Game/Geometry/Meshes/Items/Shotgun/Anims/Reload/AM_Shotgun_Reload2.AM_Shotgun_Reload2" :`5` "/Game/Geometry/Meshes/Items/Shotgun/Anims/Reload/AM_Shotgun_Reload1.AM_Shotgun_Reload1" :`6` null :!type "AnimMontage Object Reference"))
        (:`then`
          (if _outsuccess
            (bind _returnvalue_2 (`self.Reload` (select `int` _bullets :`0` "/Game/Geometry/Meshes/Player/Anims/Shotgun/Reloading/AM_ShotgunReloadFull.AM_ShotgunReloadFull" :`1` "/Game/Geometry/Meshes/Player/Anims/Shotgun/Reloading/AM_ShotgunReload5.AM_ShotgunReload5" :`2` "/Game/Geometry/Meshes/Player/Anims/Shotgun/Reloading/AM_ShotgunReload4.AM_ShotgunReload4" :`3` "/Game/Geometry/Meshes/Player/Anims/Shotgun/Reloading/AM_ShotgunReload3.AM_ShotgunReload3" :`4` "/Game/Geometry/Meshes/Player/Anims/Shotgun/Reloading/AM_ShotgunReload2.AM_ShotgunReload2" :`5` "/Game/Geometry/Meshes/Player/Anims/Shotgun/Reloading/AM_ShotgunReload1.AM_ShotgunReload1" :`6` null :!type "AnimMontage Object Reference") 1.0 0.0 true 1))
            (if _returnvalue_2
              (`self.DetermineBulletVisibility`))))))))

(event `DetermineBulletVisibility`
  (bind (_outitem _returnvalue) (`self.GetShootItem`))
  (bind _bullets (`ShootItem.Bullets` _outitem))
  (if _returnvalue
    (`SceneComponent.SetVisibility` (`self.Bullet1`) (> _bullets 1) false)
    (`SceneComponent.SetVisibility` (`self.Bullet2`) (> _bullets 2) false)
    (`SceneComponent.SetVisibility` (`self.EjectBullet`) (> _bullets 0) false)))

(fn `GetMesh`
  (returns (ReturnValue :type "SceneComponent Object Reference"))
  (return (`self.ViewmodelSkeletalMesh`)))

(fn `GetViewmodelData`
  (returns (ReturnValue :type "ViewmodelData Structure"))
  (return (`ViewmodelSkeletalMeshComponent.GetViewmodelData` (`self.ViewmodelSkeletalMesh`))))

(fn `UserConstructionScript`
  (`parent.UserConstructionScript`))