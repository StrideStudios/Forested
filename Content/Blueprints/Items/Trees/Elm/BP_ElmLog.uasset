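; Elm log item that defines its data through property getters: stacking, fire fuel value, inventory render actor and chop-stump setup as a full log.
; Its world actor properties use TreeItemActor with a static mesh override from GetLogMesh.
; GetLogMesh holds an unconnected selection between the in-hand trunk when picked up and elm trunk variants by saved tree index.
; The UI icon is set to an IES texture.
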(fn `GetChopStumpProperties`
  (returns (TreeLogType :type "ETreeLogType Enum") (StaticMesh :type "StaticMesh Soft Object Reference"))
  (return "Full" "/Game/Geometry/Meshes/Items/Trees/SM_TrunkInHand.SM_TrunkInHand"))

(fn `GetFireFuelProperties`
  (returns (BurnTime :type "Float (double-precision)"))
  (return 150.0))

(fn `GetItemActorProperties`
  (returns (ReturnValue :type "ItemActorProperties Structure"))
  (bind _returnvalue (`ItemActorSpawnAsyncAction.SetOverrideStaticMesh` (make `ItemActorProperties` "/Script/Forested.TreeItemActor" 100.0) (`self.GetLogMesh`)))
  (return _returnvalue))

(fn `GetPlayerInventoryProperties`
  (returns (InventoryRenderClass :type "PlayerInventoryActor Soft Class Reference") (StaticMesh :type "StaticMesh Soft Object Reference"))
  (return "/Game/Blueprints/Items/Trees/Elm/BP_ElmLogPlayerInventoryActor.BP_ElmLogPlayerInventoryActor_C" null))

(fn `GetProperties`
  (returns (ReturnValue :type "ItemProperties Structure"))
  (return (make `ItemProperties` "Elm Log" 5 "/Engine/EngineLightProfiles/90Degree_IES.90Degree_IES")))