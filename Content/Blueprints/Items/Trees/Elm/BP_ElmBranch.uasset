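; Elm Branch item definition that supplies the name, small stack limit and placeholder-looking UI texture for a stackable tree item.
; Its world actor uses the TreeItemActor class with a static mesh override from GetBranchMesh, and its inventory rendering uses a dedicated elm branch actor.
; The GetBranchMesh graph holds only unused logic for choosing an in-hand mesh after pickup or an elm leaves variant by saved tree index.
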(fn `GetItemActorProperties`
  (returns (ReturnValue :type "ItemActorProperties Structure"))
  (bind _returnvalue (`ItemActorSpawnAsyncAction.SetOverrideStaticMesh` (make `ItemActorProperties` "/Script/Forested.TreeItemActor") (`self.GetBranchMesh`)))
  (return _returnvalue))

(fn `GetPlayerInventoryProperties`
  (returns (InventoryRenderClass :type "PlayerInventoryActor Soft Class Reference") (StaticMesh :type "StaticMesh Soft Object Reference"))
  (return "/Game/Blueprints/Items/Trees/Elm/BP_ElmBranchPlayerInventoryActor.BP_ElmBranchPlayerInventoryActor_C" null))

(fn `GetProperties`
  (returns (ReturnValue :type "ItemProperties Structure"))
  (return (make `ItemProperties` "Elm Branch" 3 "/Engine/EngineMaterials/DefaultCalibrationColor.DefaultCalibrationColor")))