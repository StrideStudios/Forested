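; Player inventory actor for the axe: handles hatchet swings, the right-interact pose and a raised pose near obstructions.
; Left interact plays a horizontal or, while right is held, vertical swing.
; PauseMontage notifies freeze montages; releasing right, or a vertical swing blending out without it, resumes or stops the right-interact montage.
; InventoryTick sphere-checks beside the camera, starting the hatchet-up montage when blocked and resuming it when clear.
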(event `self.ReceiveOnLeftInteract`
  (params (IsMontagePlaying :type Boolean))
  (if (`PlayerInputComponent.IsHoldingRightInteract` (`FPlayer.PlayerInputComponent` (`LevelDefaults.GetPlayer`)))
    (`self.Swing` "/Game/Geometry/Meshes/Player/Anims/Axe/AM_HatchetVerticalSwing.AM_HatchetVerticalSwing" (`ForestedLibrary.MakeAlphaBlend` null "HermiteCubic" 0.6))
    (else
      (`self.Swing` "/Game/Geometry/Meshes/Player/Anims/Axe/AM_HatchetSwing.AM_HatchetSwing" (`ForestedLibrary.MakeAlphaBlend` null "HermiteCubic" 0.6)))))

(event `self.ReceiveOnRightInteract`
  (params (IsMontagePlaying :type Boolean))
  (`self.StartMontage` "/Game/Geometry/Meshes/Player/Anims/Axe/AM_HatchetRightInteract.AM_HatchetRightInteract"))

(event `EndAnim`
  (params (Montage :type "AnimMontage Object Reference"))
  (if (== Montage "/Game/Geometry/Meshes/Player/Anims/Axe/AM_HatchetRightInteract.AM_HatchetRightInteract")
    (bind _returnvalue (`self.ResumeMontage` Montage))
    (if (not _returnvalue)
      (`self.StopMontage` 0.25 Montage))))

(event `self.ReceiveOnMontageNotifyBegin`
  (params (Montage :type "AnimMontage Object Reference") (Notify :type Name))
  (if (== Notify "PauseMontage")
    (`self.PauseMontage` Montage)))

(event `self.ReceiveInventoryTick`
  (params (DeltaTime :type "Float (single-precision)"))
  (bind _returnvalue (`AnimInstance.GetCurrentActiveMontage` (`self.GetPlayerAnimInstance`)))
  (bind _camera (`FPlayer.Camera` (`LevelDefaults.GetPlayer`)))
  (bind _returnvalue_2 (+ (+ (`SceneComponent.K2_GetComponentLocation` _camera) (* (`SceneComponent.GetRightVector` _camera) 20.0)) (* (`SceneComponent.GetForwardVector` _camera) 30.0)))
  (bind (_outhit _returnvalue_3) (`KismetSystemLibrary.SphereTraceSingle` _returnvalue_2 _returnvalue_2 20.0 "TraceTypeQuery1" true))
  (if _returnvalue_3
    (`self.StartMontage` "/Game/Geometry/Meshes/Player/Anims/Axe/AM_HatchetUp.AM_HatchetUp")
    (elif (== _returnvalue "/Game/Geometry/Meshes/Player/Anims/Axe/AM_HatchetUp.AM_HatchetUp")
      (`self.ResumeMontage` _returnvalue))))

(event `self.ReceiveOnRightEndInteract`
  (params (IsMontagePlaying :type Boolean))
  (`self.EndAnim` (`PlayerAnimInstance.GetCurrentActiveMontageOfGroup` (`self.GetPlayerAnimInstance`) "PrimaryGroup")))

(event `self.ReceiveOnMontageBlendOut`
  (params (Montage :type "AnimMontage Object Reference") (bInterrupted :type Boolean))
  (if (== Montage "/Game/Geometry/Meshes/Player/Anims/Axe/AM_HatchetVerticalSwing.AM_HatchetVerticalSwing")
    (if (not (`PlayerInputComponent.IsHoldingRightInteract` (`FPlayer.PlayerInputComponent` (`LevelDefaults.GetPlayer`))))
      (`self.EndAnim` (`PlayerAnimInstance.GetCurrentActiveMontageOfGroup` (`self.GetPlayerAnimInstance`) "PrimaryGroup")))))

(fn `UserConstructionScript`)