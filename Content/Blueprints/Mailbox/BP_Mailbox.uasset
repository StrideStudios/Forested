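; BP_Mailbox is an interactable mailbox actor the player can open and close with animated first-person arms.
; Opening eases the player to a set spot, plays door and arm animations, then blends the view to the mailbox.
; Closing plays reverse animations, and an EndAnim montage notify blends back to the player, restoring inventory selection, HUD and game focus.
; Selection requires close range and facing the mailbox front.
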(event `self.OpenMailbox`
  (`InterpolatePlayerAsyncAction.InterpolatePlayerTo` (`LevelDefaults.GetPlayer`) (`SceneComponent.K2_GetComponentToWorld` (`self.PlayerLocation`)) 0.35 "SinusoidalInOut"
    (:`then`
      (`TimedEventAsyncAction.AddTimedEvent` 0.25
        (:`Complete`
          (`SkeletalMeshComponent.PlayAnimation` (`self.DoorFlag`) "/Game/Geometry/Meshes/Mailbox/AS_DoorOpenMailboxFlag.AS_DoorOpenMailboxFlag" false)
          (`|PlayMontage` (`self.PlayerArms`) "/Game/Geometry/Meshes/Mailbox/AM_ArmsOpenMailbox.AM_ArmsOpenMailbox"
            (:`then`
              (`FrameDelayAsyncAction.AddFrameDelay`
                (:`Complete`
                  (`PlayerController.SetViewTargetWithBlend` (`FPlayer.GetPlayerController` (`LevelDefaults.GetPlayer`)) self 0.25 "VTBlend_Linear" 0.0 false))))))))))

(event `self.CloseMailbox`
  (bind _returnvalue (`LevelDefaults.GetPlayer`))
  (bind _returnvalue_2 (`LevelDefaults.GetPlayer`))
  (`SkeletalMeshComponent.PlayAnimation` (`self.DoorFlag`) "/Game/Geometry/Meshes/Mailbox/AS_DoorCloseMailboxFlag.AS_DoorCloseMailboxFlag" false)
  (bind _notifyname (`|PlayMontage` (`self.PlayerArms`) "/Game/Geometry/Meshes/Mailbox/AM_ArmsCloseMailbox.AM_ArmsCloseMailbox")
    (:`OnNotifyBegin`
      (if (== _notifyname "EndAnim")
        (`PlayerController.SetViewTargetWithBlend` (`FPlayer.GetPlayerController` _returnvalue_2) _returnvalue_2 0.15 "VTBlend_Linear" 0.0 true)
        (`TimedEventAsyncAction.AddTimedEvent` 0.15
          (:`Complete`
            (`PlayerInventory.ResetSelectedItem` (`FPlayer.PlayerInventory` _returnvalue))
            (`PlayerHud.ShowHud` (`FPlayer.GetHud` _returnvalue))
            (`FPlayer.SetGameFocus` _returnvalue)))))))

(fn `CanSelect`
  (params (Player :type "FPlayer Object Reference") (HitResult :type "HitResult Structure (by ref)") (HeldTime :type "Float (double-precision)"))
  (returns (ReturnValue :type Boolean))
  (return (and (< (`KismetMathLibrary.DotProduct2D` (`KismetMathLibrary.Conv_VectorToVector2D` (`SceneComponent.GetForwardVector` (`FPlayer.Camera` Player))) (`KismetMathLibrary.Conv_VectorToVector2D` (`self.GetActorForwardVector`))) -0.5) (<= (`.Distance` (`GameplayStatics.BreakHitResult` HitResult)) 175.0))))

(fn `UserConstructionScript`)