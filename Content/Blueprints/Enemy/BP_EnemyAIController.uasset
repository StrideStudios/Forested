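; AI controller for BP_Enemy that chases the player and has the enemy's spawner despawn it beyond a distance limit.
; Tick sets walk speed from player distance, camera view and, at longer range, movement direction, switching to a fast nav filter up close.
; AIMoveTo drives the chase, and reaching the player starts an AttackDelay pause.
; The enemy is smoothly aligned every tick, and instantly before despawning.
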(event `self.ReceivePossess`
  (params (PossessedPawn :type "Pawn Object Reference"))
  (bind _asbp_enemy (cast `/Game/Blueprints/Enemy/BP_Enemy` PossessedPawn))
  (set `self.Enemy` _asbp_enemy))

(event `self.ReceiveTick`
  (params (DeltaSeconds :type "Float (single-precision)"))
  (bind _enemy (`self.Enemy`))
  (bind _returnvalue (< (`self.GetDistanceToPlayer`) 5000.0))
  (bind _camera (`FPlayer.Camera` (`LevelDefaults.GetPlayer`)))
  (bind _enemyspawner (`/Game/Blueprints/Enemy/BP_Enemy.EnemySpawner` _enemy))
  (bind _returnvalue_2 (`KismetMathLibrary.Dot_VectorVector` (`KismetMathLibrary.GetDirectionUnitVector` (`self.K2_GetActorLocation` (`self.Enemy`)) (`self.K2_GetActorLocation` (`LevelDefaults.GetPlayer`))) (`KismetMathLibrary.Normal` (`self.GetVelocity` (`self.Enemy`)))))
  (bind _returnvalue_3 (>= (`KismetMathLibrary.Dot_VectorVector` (`SceneComponent.GetForwardVector` _camera) (`KismetMathLibrary.GetDirectionUnitVector` (`SceneComponent.K2_GetComponentLocation` _camera) (`self.K2_GetActorLocation` (`self.Enemy`)))) 0.65))
  (set `self.Delta Seconds` DeltaSeconds)
  (`|ExecutionSequence`
    (:`then_0`
      (if (> (`self.AttackDelay`) 0.0)
        (set `self.AttackDelay` (- (`self.AttackDelay`) (`self.Delta Seconds`)))
        (elif (and (`KismetSystemLibrary.IsValid` _enemy) (`KismetSystemLibrary.IsValid` _enemyspawner))
          (if (<= (`self.GetDistanceToPlayer`) (`/Game/Blueprints/Enemy/BP_EnemySpawner.DistanceForDespawn` _enemyspawner))
            (set `CharacterMovementComponent.MaxWalkSpeed` (`KismetMathLibrary.SelectFloat` (`KismetMathLibrary.SelectFloat` 800.0 600.0 _returnvalue_3) (* (* (`KismetMathLibrary.SelectFloat` 1.0 5.0 _returnvalue_3) (`KismetMathLibrary.MapRangeClamped` (`self.GetDistanceToPlayer`) 7500.0 25000.0 1.0 50.0)) (`KismetMathLibrary.SelectFloat` (`KismetMathLibrary.MapRangeClamped` _returnvalue_2 0.0 1.0 0.0 0.75) (`KismetMathLibrary.MapRangeClamped` _returnvalue_2 0.0 250100.0 0.5 1.0) _returnvalue_3)) _returnvalue) (`Character.CharacterMovement` (`self.Enemy`)))
            (set `self.DefaultNavigationFilterClass` (select `bool` _returnvalue :`false` "/Script/AIModule.NavFilter_AIControllerDefault" :`true` "/Game/Blueprints/Enemy/BP_FastNavFilter.BP_FastNavFilter_C" :!type "NavigationQueryFilter Class Reference"))
            (`|AIMoveTo` (`self.Enemy`) (0.0 0.0 0.0) (`LevelDefaults.GetPlayer`) 80.0 true
              (:`OnSuccess`
                (set `self.AttackDelay` 1.5)))
            (else
              (`/Game/Blueprints/Enemy/BP_Enemy.Align` (`self.Enemy`) true 0.0 1.0)
              (`/Game/Blueprints/Enemy/BP_EnemySpawner.DespawnInstance` (`/Game/Blueprints/Enemy/BP_Enemy.EnemySpawner` (`self.Enemy`)) (`self.Enemy`)))))))
    (:`then_1`
      (`/Game/Blueprints/Enemy/BP_Enemy.Align` (`self.Enemy`) false (`self.Delta Seconds`) 2.5))))

(fn `GetDistanceToPlayer`
  (returns (Distance :type "Float (double-precision)"))
  (return (`KismetMathLibrary.SelectFloat` (`KismetMathLibrary.Vector_Distance` (`self.K2_GetActorLocation` (`LevelDefaults.GetPlayer`)) (`self.K2_GetActorLocation` (`self.Enemy`))) 1000000000.0 (`KismetSystemLibrary.IsValid` (`LevelDefaults.GetPlayer`)))))

(fn `UserConstructionScript`)