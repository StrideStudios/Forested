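; Enemy spawner that scatters randomly scaled and rotated BP_Enemy actors, each with a default controller, on navigable ground at BeginPlay.
; Random points in the Bounding volume drive downward traces, and hits that project onto the navmesh become spawn locations.
; DespawnInstance and RespawnInstance swap enemies for mesh instances and back, though neither is called here.
; The TreeType-keyed Meshes map is set empty, and respawn assigns no controller or TreeType.
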(event `self.ReceiveBeginPlay`
  (`self.SpawnEntities`)
  (set `self.Meshes` (`|MakeMap` 0 :!type "Byte" :!valuetype "HierarchicalInstancedStaticMeshComponent Object Reference")))

(event `self.ReceiveTick`
  (params (DeltaSeconds :type "Float (single-precision)")))

(fn `DespawnInstance`
  (params (Enemy :type "/Game/Blueprints/Enemy/BP_Enemy Object Reference"))
  (`InstancedStaticMeshComponent.AddInstanceWorldSpace` (`BlueprintMapLibrary.Map_Find` (`self.Meshes`) (`/Game/Blueprints/Enemy/BP_Enemy.TreeType` Enemy)) (`KismetMathLibrary.MakeTransform` (- (.location (`self.GetTransform` Enemy)) (* (0.0 0.0 750.0) (`/Game/Blueprints/Enemy/BP_Enemy.SetScale` Enemy))) (.rotation (`self.GetTransform` Enemy)) (.scale (`self.GetTransform` Enemy))))
  (`self.K2_DestroyActor` Enemy))

(fn `RespawnInstance`
  (params (Mesh :type "HierarchicalInstancedStaticMeshComponent Object Reference") (Index :type Integer))
  (bind _x (.x (.scale (`InstancedStaticMeshComponent.GetInstanceTransform` Mesh Index true))))
  (bind _returnvalue (`|SpawnActorFromClass` "/Game/Blueprints/Enemy/BP_Enemy.BP_Enemy_C" (`KismetMathLibrary.MakeTransform` (+ (.location (`InstancedStaticMeshComponent.GetInstanceTransform` Mesh Index true)) (* (0.0 0.0 750.0) _x)) (.rotation (`InstancedStaticMeshComponent.GetInstanceTransform` Mesh Index true)) (`KismetMathLibrary.Conv_DoubleToVector` _x)) "AlwaysSpawn" "OverrideRootScale" null null))
  (set `/Game/Blueprints/Enemy/BP_Enemy.SetScale` _x _returnvalue)
  (`InstancedStaticMeshComponent.RemoveInstance` Mesh Index))

(fn `SpawnEntities`
  (locals (Index :type Integer) (Scale :type "Float (double-precision)"))
  (bind _bounding (`self.Bounding`))
  (bind _returnvalue (`KismetMathLibrary.RandomPointInBoundingBox` (`SceneComponent.K2_GetComponentLocation` _bounding) (`BoxComponent.GetScaledBoxExtent` _bounding)))
  (for _index (range 1 (+ (`self.SpawnAmount`) 1))
    (set `local.Index` _index)
    (bind (_outhit _returnvalue_2) (`KismetSystemLibrary.LineTraceSingleForObjects` _returnvalue (- _returnvalue (0.0 0.0 75000.0)) (`|MakeArray` "ObjectTypeQuery7" :!type "EObjectTypeQuery Enum") true))
    (bind (_projectedlocation _returnvalue_3) (`NavigationSystemV1.K2_ProjectPointToNavigation` (`.Location` (`GameplayStatics.BreakHitResult` _outhit)) null null (40.0 40.0 40.0)))
    (if (and _returnvalue_2 _returnvalue_3)
      (if true
        (bind _output_get (set `local.Scale` (`KismetMathLibrary.RandomFloatInRange` 1.0 2.0)))
        (bind _returnvalue_4 (`|SpawnActorFromClass` "/Game/Blueprints/Enemy/BP_Enemy.BP_Enemy_C" (`KismetMathLibrary.MakeTransform` (+ (+ (* (0.0 0.0 750.0) _output_get) _projectedlocation) (0.0 0.0 200.0)) (`KismetMathLibrary.MakeRotator` 0.0 0.0 (`KismetMathLibrary.RandomFloatInRange` -180.0 180.0)) (`KismetMathLibrary.Conv_DoubleToVector` (`local.Scale`))) "AlwaysSpawn" "OverrideRootScale" null null))
        (`Pawn.SpawnDefaultController` _returnvalue_4)
        (set `/Game/Blueprints/Enemy/BP_Enemy.SetScale` (`local.Scale`) _returnvalue_4)))))

(fn `UserConstructionScript`)