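; BP_Enemy is an enemy actor that tilts to match the ground beneath it and registers gun hits.
; BeginPlay stores its origin and spawner, and randomizes a custom primitive data value on the mesh.
; Gun damage is mapped to a HitDelay timer that Tick counts down.
; The construction script calls Align, which traces downward and instantly fits capsule pitch and roll to the surface normal, keeping yaw, with optional interpolation.
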(event `self.ReceiveBeginPlay`
  (set `self.Origin` (`self.K2_GetActorLocation`))
  (`PrimitiveComponent.SetCustomPrimitiveDataFloat` (`self.StaticMesh`) 0 (`KismetMathLibrary.RandomFloatInRange` 0.0 2.0))
  (bind _returnvalue (`GameplayStatics.GetActorOfClass` "/Game/Blueprints/Enemy/BP_EnemySpawner.BP_EnemySpawner_C"))
  (set `self.EnemySpawner` _returnvalue))

(event `DamageableInterface.Damage`
  (params (Player :type "FPlayer Object Reference") (HitResult :type "HitResult Structure (by ref)") (Damage :type "Float (single-precision)") (DamageType :type "EDamageType Enum" :default "Basic"))
  (if (`|EnumEquality` DamageType "Gun")
    (`KismetSystemLibrary.PrintString` (`KismetStringLibrary.Conv_DoubleToString` Damage))
    (set `self.HitDelay` (`KismetMathLibrary.MapRangeClamped` Damage 15.0 25.0 0.0 0.75))))

(event `self.ReceiveTick`
  (params (DeltaSeconds :type "Float (single-precision)"))
  (set `self.HitDelay` (- (`self.HitDelay`) DeltaSeconds)))

(fn `Align`
  (params (InInstant :type Boolean) (InDeltaTime :type "Float (double-precision)") (InSpeed :type "Float (double-precision)"))
  (locals (Instant :type Boolean) (DeltaTime :type "Float (double-precision)") (Speed :type "Float (double-precision)"))
  (bind _returnvalue (`self.K2_GetActorLocation`))
  (bind _capsulecomponent (`self.CapsuleComponent`))
  (bind _returnvalue_2 (`SceneComponent.K2_GetComponentRotation` _capsulecomponent))
  (set `local.Instant` InInstant)
  (set `local.DeltaTime` InDeltaTime)
  (set `local.Speed` InSpeed)
  (bind (_outhit _returnvalue_3) (`KismetSystemLibrary.LineTraceSingle` _returnvalue (- _returnvalue (* (0.0 0.0 1.0) (* (`self.SetScale`) 1000.0))) "TraceTypeQuery1" false (`|MakeArray` (`self.EnemySpawner`) :!type "Actor Object Reference") "ForDuration"))
  (bind _returnvalue_4 (`KismetMathLibrary.SelectVector` (`.ImpactNormal` (`GameplayStatics.BreakHitResult` _outhit)) (0.0 0.0 1.0) _returnvalue_3))
  (bind _returnvalue_5 (`KismetMathLibrary.MakeRotator` (.roll (`KismetMathLibrary.MakeRotFromZX` _returnvalue_4 (`SceneComponent.GetForwardVector` _capsulecomponent))) (.pitch (`KismetMathLibrary.MakeRotFromYZ` (`SceneComponent.GetRightVector` _capsulecomponent) _returnvalue_4)) (.yaw _returnvalue_2)))
  (bind _returnvalue_6 (`KismetMathLibrary.SelectRotator` _returnvalue_5 (`KismetMathLibrary.RInterpTo` _returnvalue_2 _returnvalue_5 (`local.DeltaTime`) (`local.Speed`)) (`local.Instant`)))
  (`KismetSystemLibrary.PrintString` (`KismetStringLibrary.Conv_RotatorToString` _returnvalue_6))
  (`SceneComponent.K2_SetWorldRotation` _capsulecomponent _returnvalue_6 false false))

(fn `UserConstructionScript`
  (`self.Align` true))