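; BP_FPlayer is the player Blueprint, holding debug controls for the day/night cycle.
; The left and right bracket keys find the Sky actor, halve or double its seconds per day and per night, and print the new values.
; An unwired chain that would fill PlayerInventory slots with an axe, shotgun, elm log halves and lighter never runs, as BeginPlay and the construction script are empty.
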(event `Key|LeftBracket`
  (params (Key :type "Key Structure"))
  (:`Pressed`
    (bind _returnvalue (`GameplayStatics.GetActorOfClass` "/Script/Forested.Sky"))
    (bind _output_get (set `Sky.DayTimeSpeedInSecondsPerDay` (/ (`Sky.DayTimeSpeedInSecondsPerDay` _returnvalue) 2.0) _returnvalue))
    (`KismetSystemLibrary.PrintString` (`KismetStringLibrary.Conv_DoubleToString` _output_get))
    (bind _output_get_2 (set `Sky.NightTimeSpeedInSecondsPerNight` (/ (`Sky.NightTimeSpeedInSecondsPerNight` _returnvalue) 2.0) _returnvalue))
    (`KismetSystemLibrary.PrintString` (`KismetStringLibrary.Conv_DoubleToString` _output_get_2))))

(event `Key|RightBracket`
  (params (Key :type "Key Structure"))
  (:`Pressed`
    (bind _returnvalue (`GameplayStatics.GetActorOfClass` "/Script/Forested.Sky"))
    (bind _output_get (set `Sky.DayTimeSpeedInSecondsPerDay` (* (`Sky.DayTimeSpeedInSecondsPerDay` _returnvalue) 2.0) _returnvalue))
    (`KismetSystemLibrary.PrintString` (`KismetStringLibrary.Conv_DoubleToString` _output_get))
    (bind _output_get_2 (set `Sky.NightTimeSpeedInSecondsPerNight` (* (`Sky.NightTimeSpeedInSecondsPerNight` _returnvalue) 2.0) _returnvalue))
    (`KismetSystemLibrary.PrintString` (`KismetStringLibrary.Conv_DoubleToString` _output_get_2))))

(event `self.ReceiveBeginPlay`)

(fn `UserConstructionScript`)